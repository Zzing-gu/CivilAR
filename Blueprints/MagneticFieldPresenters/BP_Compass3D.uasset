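; BP_Compass3D is a magnetic field presenter that acts as a 3D compass, turning its arrow to follow the reported field.
; It attaches to and detaches from a magnetic field engine notifier, which drives its updates.
; Each update caches the vector and, unless the player's BP_ARPawn is Fixed, sets the root's world rotation via look-at toward the field's X/Y, ignoring Z to keep it horizontal.
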(event EventNotifyUpdatedMagneticFieldEvent
  (params (MagneticField :type Vector :default "0, 0, 0"))
  ;[1 1 1] On magnetic field update, we process the change according to this actor's responsibility.
  (CallFunction|ProcessUpdatedMagneticField MagneticField))

(fn ConstructionScript)

(fn Attachto
  (params (MagneticFieldEngineNotifier :type BPI%20Observable%20Magnetic%20Field%20Interface))
  ;[1 1 1] Attach this object/blueprint to the magnetic field engine which will drive updates.
  (Default|Attach MagneticFieldEngineNotifier self)
  (Utilities|MagneticFieldLogDebug (Variables|Debug|GetDebug) "Attached to" (Utilities|GetDisplayName (Utilities|ToObject(Interface) MagneticFieldEngineNotifier))
    (:Exec%20Out
      (return false))))

(fn Detachfrom
  (params (MagneticFieldEngineNotifier :type BPI%20Observable%20Magnetic%20Field%20Interface))
  ;[1 1 1] Detach this object/blueprint from the location engine which was driving updates.
  (Default|Detach MagneticFieldEngineNotifier self)
  (Utilities|MagneticFieldLogDebug (Variables|Debug|GetDebug) "Detached from" (Utilities|GetDisplayName (Utilities|ToObject(Interface) MagneticFieldEngineNotifier))
    (:Exec%20Out
      (return false))))

(fn ProcessUpdatedMagneticField
  (params (MagneticField :type Vector :default "0, 0, 0"))
  (Variables|MagneticField|SetLastKnownMagneticField MagneticField)
  (bind _asbp_arpawn (Utilities|Casting|CastToBP_ARPawn (Game|Player|GetPlayerPawn 0)))
  (if (not (Variables|/Game/HandheldARBP/Blueprints/GameFramework/BP_ARPawn.BP_ARPawn_C|Getfixed _asbp_arpawn))
    (Transformation|SetWorldRotation (Variables|Default|GetDefaultSceneRoot) (Math|Rotator|FindLookatRotation (Math|Vector|MakeVector 0.0 0.0 0.0) (Math|Vector|MakeVector (* 1 (.X (Math|Vector|BreakVector (Variables|MagneticField|GetLastKnownMagneticField)))) (* 1 (.Y (Math|Vector|BreakVector (Variables|MagneticField|GetLastKnownMagneticField)))) 0.0)) false false)))